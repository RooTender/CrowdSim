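; Chaos box truck vehicle that drives itself along the spline of the first Path actor found in the level, at constant throttle set on BeginPlay.
; Each tick, GetPath aims at the spline point nearest a look-ahead position along the local tangent, mapping the yaw difference to clamped steering.
; PushBreakOnTurn adds a slight fixed brake when steering is sharp and forward speed exceeds a threshold.
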(event EventTick
  (params (DeltaSeconds :type Float%20%28single-precision%29))
  (bind _vehiclemovementcomponent (Variables|Default|GetVehicleMovementComponent))
  (bind _outactors (Actor|GetAllActorsOfClass "/Game/VehicleVarietyVol2/Blueprints/Path.Path_C"))
  (bind _steering (CallFunction|GetPath _outactors (Variables|Default|GetSensitivity%20angle)))
  (Class|ChaosVehicleMovementComponent|SetSteeringInput _vehiclemovementcomponent _steering)
  (bind _break (CallFunction|PushBreakonTurn _steering (Vehicle|GetForwardSpeed _vehiclemovementcomponent)))
  (Class|ChaosVehicleMovementComponent|SetBrakeInput _vehiclemovementcomponent _break))

(event EventBeginPlay
  (Class|ChaosVehicleMovementComponent|SetThrottleInput (Variables|Default|GetVehicleMovementComponent) 0.5))

(fn ConstructionScript)

(fn GetPath
  (params (Splines :type Array%20of%20Path%20Object%20References) (Clamp%20angle :type Float%20%28double-precision%29))
  (bind _returnvalue (Transformation|GetActorLocation))
  (bind _output (Utilities|Array|Get(acopy) Splines))
  (bind _spline (Variables|/Game/VehicleVarietyVol2/Blueprints/Path.Path_C|GetSpline _output))
  (return (Math|Float|MapRangeClamped (.yaw (Math|Rotator|Delta(Rotator) (Math|Rotator|FindLookatRotation _returnvalue (Spline|FindLocationClosesttoWorldLocation _spline (+ (* (Math|Vector|Normalize (Class|SplineComponent|FindTangentClosesttoWorldLocation _spline _returnvalue "World")) 5e+02) _returnvalue) "World")) (Transformation|GetActorRotation))) (* Clamp%20angle -1.0) Clamp%20angle -1.0 1.0)))

(fn PushBreakonTurn
  (params (Steering :type Float%20%28double-precision%29) (Vehicle%20Speed :type Float%20%28double-precision%29))
  (if (and (> (Math|Float|Absolute(Float) Steering) 0.3) (> Vehicle%20Speed 75.0))
    (return (Math|Float|Lerp 0.0 0.5 0.05))
    (else
      (return 0.0))))