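; BP_Campervan_Chaos is a self-driving campervan, apparently a Chaos wheeled vehicle, that moves without player input.
; BeginPlay applies DefaultSpeed as throttle, and each Tick hands the movement component to VehicleMovement's shared ForwardMovement routine.
; When PawnSensing sees another WheeledVehiclePawn, it calls VehicleMovement's Stop with the movement component and DefaultSpeed.
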(event OnSeePawn(PawnSensing)
  (params (Pawn :type Pawn%20Object%20Reference))
  (Utilities|Casting|CastToWheeledVehiclePawn Pawn)
  (Default|Stop (Variables|Default|GetVehicle%20Movement) (Variables|Default|GetVehicleMovementComponent) (Variables|Default|GetDefault%20Speed)))

(event EventTick
  (params (DeltaSeconds :type Float%20%28single-precision%29))
  (Default|ForwardMovement (Variables|Default|GetVehicle%20Movement) 0.0 (Variables|Default|GetVehicleMovementComponent) self))

(event EventBeginPlay
  (Class|ChaosVehicleMovementComponent|SetThrottleInput (Variables|Default|GetVehicleMovementComponent) (Variables|Default|GetDefault%20Speed)))

(fn ConstructionScript)