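; VehicleMovement steers a wheeled vehicle along a spline path through its ForwardMovement event.
; GetPath projects 500 units along the tangent of the first Path actor's spline, snaps that point to the spline, and maps the look-at yaw difference to clamped steering using SensitivityAngle.
; PushBreakOnTurn receives steering and forward speed to set brake input, but is a stub returning zero.
; All Path actors are fetched on every call.
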(event Custom|ForwardMovement
  (params (DeltaSeconds :type Float%20%28single-precision%29) (Vehicle%20Movement%20Component :type Chaos%20Vehicle%20Movement%20Component%20Object%20Reference) (Pawn%20reference :type Pawn%20Object%20Reference))
  (bind _outactors (Actor|GetAllActorsOfClass "/Game/VehicleVarietyVol2/Blueprints/Path.Path_C"))
  (bind _steering (CallFunction|GetPath Pawn%20reference _outactors (Variables|Default|GetSensitivity%20angle)))
  (Class|ChaosVehicleMovementComponent|SetSteeringInput Vehicle%20Movement%20Component _steering)
  (bind _break (CallFunction|PushBreakonTurn _steering (Vehicle|GetForwardSpeed Vehicle%20Movement%20Component)))
  (Class|ChaosVehicleMovementComponent|SetBrakeInput Vehicle%20Movement%20Component _break))

(fn PushBreakonTurn
  (params (Steering :type Float%20%28double-precision%29) (Vehicle%20Speed :type Float%20%28double-precision%29))
  (return 0.0))

(fn GetPath
  (params (Pawn%20reference :type Pawn%20Object%20Reference) (Splines :type Array%20of%20Path%20Object%20References) (Clamp%20angle :type Float%20%28double-precision%29))
  (bind _returnvalue (Transformation|GetActorLocation Pawn%20reference))
  (bind _output (Utilities|Array|Get(acopy) Splines))
  (bind _spline (Variables|/Game/VehicleVarietyVol2/Blueprints/Path.Path_C|GetSpline _output))
  (return (Math|Float|MapRangeClamped (.yaw (Math|Rotator|Delta(Rotator) (Math|Rotator|FindLookatRotation _returnvalue (Spline|FindLocationClosesttoWorldLocation _spline (+ (* (Math|Vector|Normalize (Class|SplineComponent|FindTangentClosesttoWorldLocation _spline _returnvalue "World")) 5e+02) _returnvalue) "World")) (Transformation|GetActorRotation Pawn%20reference))) (* Clamp%20angle -1.0) Clamp%20angle -1.0 1.0)))